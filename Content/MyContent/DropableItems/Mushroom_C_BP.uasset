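; Droppable mushroom actor that the player collects on Interact when CanPickup is set, up to a limit of ten held.
; Pickup notifies the Spore2ScoreCharacter, destroys the actor and plays a sound, or prints a full-inventory message.
; BeginPlay registers the actor with its Mysellium widget; the overlap logic to show, hide and camera-face it is disconnected.
; Health and nutrient functions remain stubs using zero values.
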(event `RotateToFacePlayer`
  ;[1 1 1] Rotate Health Widget to face Player
  (bind _asspore_2score_character (cast `/Game/MyContent/Characters/Blueprints/Spore2ScoreCharacter` (`GameplayStatics.GetPlayerCharacter` 0)))
  (`SceneComponent.K2_SetWorldRotation` (`self.Widget`) (`KismetMathLibrary.FindLookAtRotation` (`SceneComponent.K2_GetComponentLocation` (`self.DefaultSceneRoot`)) (`SceneComponent.K2_GetComponentLocation` (`/Game/MyContent/Characters/Blueprints/Spore2ScoreCharacter.FollowCamera` _asspore_2score_character))) false false))

(event `self.ReceiveBeginPlay`
  ;[1 1 1] BeginPlay - Get reference to Widget_BP
  (`parent.ReceiveBeginPlay`)
  (bind _asmysellium_widget_bp (cast `/Game/MyContent/Widgets/MyselliumWidget_BP` (`WidgetComponent.GetUserWidgetObject` (`self.Widget`))))
  (bind _output_get (set `self.MyselliumWidget` _asmysellium_widget_bp))
  (set `/Game/MyContent/Widgets/MyselliumWidget_BP.OwningActor` self _output_get))

(event `InputAction|Interact`
  (params (Key :type "Key Structure"))
  ;[1 1 1] Interact with Mushroom
  (:`Pressed`
    (if (`self.CanPickup`) :!label _label
      (bind _asspore_2score_character (cast `/Game/MyContent/Characters/Blueprints/Spore2ScoreCharacter` (`GameplayStatics.GetPlayerCharacter` 0)))
      (if (<= (`/Game/MyContent/Characters/Blueprints/Spore2ScoreCharacter.MushroomsHolding` _asspore_2score_character) 9)
        (`/Game/MyContent/Characters/Blueprints/Spore2ScoreCharacter.PickedUpMushroom` _asspore_2score_character)
        (`self.K2_DestroyActor`)
        (`GameplayStatics.PlaySoundAtLocation` null (`self.K2_GetActorLocation` _asspore_2score_character) (struct) 1.0 1.0 0.0 null null null)
        (else
          (`KismetSystemLibrary.PrintString` "Too many mushrooms within inventory"))))))

(event `/Game/MyContent/Interface/Score2Spore_BPI.Interact`
  ;[1 1 1] Interact with Mushroom
  (goto _label))

(event `self.SphereOfInfluence.OnComponentBeginOverlap`
  (params (OverlappedComponent :type "PrimitiveComponent Object Reference") (OtherActor :type "Actor Object Reference") (OtherComp :type "PrimitiveComponent Object Reference") (OtherBodyIndex :type Integer) (bFromSweep :type Boolean) (SweepResult :type "HitResult Structure (by ref)"))
  ;[1 1 1] Make Widget Visbile when nearby and Invisible when moving away
)

(event `self.SphereOfInfluence.OnComponentEndOverlap`
  (params (OverlappedComponent :type "PrimitiveComponent Object Reference") (OtherActor :type "Actor Object Reference") (OtherComp :type "PrimitiveComponent Object Reference") (OtherBodyIndex :type Integer))
  ;[1 1 1] Make Widget Visbile when nearby and Invisible when moving away
)

(fn `IsHealthy`
  (returns (IsHealthy :type Boolean))
  (return (>= 0.0 80.0)))

(fn `IsMaxHealth`
  (returns (isMaxHealth :type Boolean))
  (return (>= 0.0 100.0)))

(fn `PlantHealthCycle`
  (`/Game/MyContent/Environment/Mysellium/Mysellium_BP.IncreaseNutrientsMessage` (`self.Mysellium_Ref`) 0.0))

(fn `UserConstructionScript`
  (`parent.UserConstructionScript`))