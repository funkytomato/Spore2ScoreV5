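; Base Blueprint for interactable trees that share nutrients with nearby plants and a Mysellium network.
; Shortly after BeginPlay it registers as the supporting tree of plants overlapping its Mysellium influence sphere.
; Each LifeCycle, a flourishing tree feeds struggling supported plants from its own nutrients.
; When connected, it sends nutrients to Mysellium while flourishing or draws them otherwise, and flourishing also spawns mushrooms on three mesh sockets.
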(event `self.ReceiveBeginPlay`
  (`parent.ReceiveBeginPlay`)
  (`KismetSystemLibrary.Delay` 0.5)
  (bind _output_get (set `self.SupportedLife` (`PrimitiveComponent.GetOverlappingActors` (`self.MyselliumSphereOfInfluence`) "/Game/MyContent/Environment/InteractableItems/Biological/Plants/PlantMaster_BP.PlantMaster_BP_C")))
  (for _array_element _output_get
    (bind _asplant_master_bp (cast `/Game/MyContent/Environment/InteractableItems/Biological/Plants/PlantMaster_BP` _array_element))
    (bind _output_get_2 (set `/Game/MyContent/Environment/InteractableItems/Biological/BiologicalMaster_BP.SupportingTree` self _asplant_master_bp))))

(event `self.ReceiveActorBeginOverlap`
  (params (OtherActor :type "Actor Object Reference"))
  (`parent.ReceiveActorBeginOverlap` OtherActor))

(event `self.ReceiveTick`
  (params (DeltaSeconds :type "Float (single-precision)"))
  (`parent.ReceiveTick` DeltaSeconds))

(event `GrowMushroomOnTree`
  (if (not (`self.MushroomSocketAOccupied`))
    (`|SpawnActorFromClass` "/Game/MyContent/GrowableMushrooms/ThreeTreeMushrooms_BP.ThreeTreeMushrooms_BP_C" (`SceneComponent.GetSocketTransform` (`self.StaticMesh`) "MushroomSocketA" "RTS_World") "Undefined" "OverrideRootScale" null null)
    (set `self.MushroomSocketAOccupied` true))
  (if (not (`self.MushroomSocketBOccupied`))
    (`|SpawnActorFromClass` "/Game/MyContent/GrowableMushrooms/ThreeTreeMushrooms_BP.ThreeTreeMushrooms_BP_C" (`SceneComponent.GetSocketTransform` (`self.StaticMesh`) "MushroomSocketB" "RTS_World") "Undefined" "OverrideRootScale" null null)
    (set `self.MushroomSocketBOccupied` true))
  (if (not (`self.MushroomSocketCOccupied`))
    (`|SpawnActorFromClass` "/Game/MyContent/GrowableMushrooms/ThreeTreeMushrooms_BP.ThreeTreeMushrooms_BP_C" (`SceneComponent.GetSocketTransform` (`self.StaticMesh`) "MushroomSocketC" "RTS_World") "Undefined" "OverrideRootScale" null null)
    (set `self.MushroomSocketCOccupied` true)
    (else
      (`KismetSystemLibrary.PrintString` "All mushroom sockets occupied"))))

(fn `LifeCycle`
  (bind _myselliumnutrientamounttosend (`self.MyselliumNutrientAmountToSend`))
  (bind _myselliumhealthbonus (`self.MySelliumHealthBonus`))
  (`parent.LifeCycle`)
  (`|ExecutionSequence`
    (:`then_0`
      ;[1 1 1] Calculate how many nutrients can be sent to supported local life
      (for _array_element (`self.SupportedLife`)
        (bind _isflourishing (`self.Am I Flourishing`))
        (if _isflourishing
          (bind _asplant_master_bp (cast `/Game/MyContent/Environment/InteractableItems/Biological/Plants/PlantMaster_BP` _array_element)
            (:`then`
              (bind _isflourishing_2 (`self.Am I Flourishing` _asplant_master_bp))
              (if (not _isflourishing_2)
                ;;[1 1 1] Plant is improving its health with help from tree
                (`self.IncreaseNutrientsMessage` _asplant_master_bp 5.0)
                (`self.DecreaseNutrients` 5.0)
                (set `self.LocalLifeSupportTotalAmount` (+ (`self.LocalLifeSupportTotalAmount`) 5.0))))
            (:`CastFailed`
              (`KismetSystemLibrary.PrintString` "TreeMaster LifeCycle failed to cast to PlantMaster")))))
      (set `self.LocalLifeSupportTotalAmount` 0.0))
    (:`then_1`
      ;[1 1 1] Send nutrients to Mysellium if connected
      (if (`self.ConnectedToMyselliumTrail`)
        ;;[1 1 1] If connected and Flourishing, do...
        (bind _isflourishing_3 (`self.Am I Flourishing`))
        (if _isflourishing_3
          ;;[1 1 1] Send nutrients to Mysellium if Flourishing
          (`/Game/MyContent/Environment/Mysellium/Mysellium_BP.IncreaseNutrientsMessage` (`self.Mysellium_Ref`) _myselliumnutrientamounttosend)
          (`self.DecreaseNutrients` _myselliumnutrientamounttosend)
          (else
            ;;[1 1 1] Recieve nutrients from Mysellium and increase nutrients in plant
            (`/Game/MyContent/Environment/Mysellium/Mysellium_BP.DecreaseNutrientsMessage` (`self.Mysellium_Ref`) _myselliumhealthbonus)
            (`self.IncreaseNutrients` _myselliumhealthbonus)))))
    (:`then_2`
      (if (`self.IsFlourishing`)
        (`self.GrowMushroomOnTree`)))))

(fn `UserConstructionScript`
  (`parent.UserConstructionScript`))